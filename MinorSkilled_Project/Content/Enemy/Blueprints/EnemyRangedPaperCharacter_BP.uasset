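; Blueprint for a ranged Paper2D enemy character that adds floating damage-number feedback.
; On a take-damage event, SpawnDamageNumbers spawns a DamageNumbersActor_BP just above the capsule top and passes it the damage.
; A separate GetRandomLocationinNavArea event picks a random reachable navmesh point within a radius and spawns the same actor class there without a damage value.
; No attack logic is defined in these graphs.
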(event `self.OnTakeDamageEvent`
  (params (pDamage :type Integer))
  (`self.SpawnDamageNumbers` pDamage))

(event `self.GetRandomLocationInNavArea`
  (params (pRadius :type "Float (single-precision)"))
  (bind _output_get (set `self.RandomLocationOnNavArea` (`NavigationSystemV1.K2_GetRandomReachablePointInRadius` (`self.K2_GetActorLocation`) pRadius null null)))
  (`|SpawnActorFromClass` "/Game/HUD/DamageNumbersActor_BP.DamageNumbersActor_BP_C" (`KismetMathLibrary.Conv_VectorToTransform` _output_get) "Undefined" "OverrideRootScale" null 0 null))

(fn `SpawnDamageNumbers`
  (params (Damage :type Integer))
  (`|SpawnActorFromClass` "/Game/HUD/DamageNumbersActor_BP.DamageNumbersActor_BP_C" (`KismetMathLibrary.Conv_VectorToTransform` (+ (`self.K2_GetActorLocation`) (`KismetMathLibrary.MakeVector` 0.0 0.0 (`CapsuleComponent.GetScaledCapsuleHalfHeight` (`self.CapsuleComponent`))) (0.0 0.0 20.0))) "Undefined" "OverrideRootScale" null Damage null))

(fn `UserConstructionScript`)