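; Projectile Blueprint for ranged enemies that destroys itself when it hits a boundary tile of the level tilemap.
; On overlap with a Tilemap0_BP actor, it converts its world X and Z location into layer 0 tile coordinates, using tile size and actor scale with an inverted vertical axis.
; It destroys itself if that tile's user data reads "Bound"; the graphs hold no movement or damage logic.
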(event `self.ReceiveActorBeginOverlap`
  (params (OtherActor :type "Actor Object Reference"))
  (bind _astilemap_0_bp (cast `/Game/2DAssets/Tilemaps/Tilemap0_BP` OtherActor))
  (bind _tilemap (`PaperTileMapComponent.TileMap` (`PaperTileMapActor.RenderComponent` _astilemap_0_bp)))
  (if (`KismetStringLibrary.EqualEqual_StrStr` (`KismetStringLibrary.Conv_NameToString` (`TileMapBlueprintLibrary.GetTileUserData` (`PaperTileMapComponent.GetTile` (`PaperTileMapActor.RenderComponent` _astilemap_0_bp) (`KismetMathLibrary.FTrunc` (/ (.x (`self.K2_GetActorLocation`)) (* (`PaperTileMap.TileHeight` _tilemap) (.x (`self.GetActorScale3D` _astilemap_0_bp))))) (* (- (`KismetMathLibrary.FTrunc` (/ (.z (`self.K2_GetActorLocation`)) (* (`PaperTileMap.TileWidth` _tilemap) (.z (`self.GetActorScale3D` _astilemap_0_bp))))) 1) -1) 0))) "Bound")
    (`self.K2_DestroyActor`)))

(fn `UserConstructionScript`)