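; Enemy spawner actor that spawns one of four Paper2D skeleton or wizard enemy variants at its own location.
; OnSpawnRandomEnemy switches on the type index it receives, so any randomness comes from the caller.
; Each branch spawns the melee or ranged character with its behavior tree, sets the variant and behaviour activation delay, passes on the GameManager, then calls Init.
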(event `self.OnSpawnRandomEnemy`
  (params (pBehaviourDelay :type "Float (single-precision)") (pEnemyType :type Integer))
  (bind _returnvalue (`self.K2_GetActorLocation`))
  (bind _gamemanager (`self.GameManager`))
  (switch `int` pEnemyType
    (:`0`
      (bind _returnvalue_2 (`AIBlueprintHelperLibrary.SpawnAIFromClass` "/Game/Enemy/Blueprints/EnemyMeleePaperCharacter_BP.EnemyMeleePaperCharacter_BP_C" "/Game/Enemy/EnemyMeleeBT.EnemyMeleeBT" _returnvalue))
      (bind _asenemy_melee_paper_character_bp (cast `/Game/Enemy/Blueprints/EnemyMeleePaperCharacter_BP` _returnvalue_2))
      (set `EnemyPaperCharacter.TypeOfEnemy` "MeleeSkeleton" _asenemy_melee_paper_character_bp)
      (set `EnemyPaperCharacter.behaviourActivationDelay` pBehaviourDelay _asenemy_melee_paper_character_bp)
      (`EnemyPaperCharacter.SetGameManager` _asenemy_melee_paper_character_bp _gamemanager)
      (`EnemyPaperCharacter.Init` _asenemy_melee_paper_character_bp))
    (:`1`
      (bind _returnvalue_3 (`AIBlueprintHelperLibrary.SpawnAIFromClass` "/Game/Enemy/Blueprints/EnemyMeleePaperCharacter_BP.EnemyMeleePaperCharacter_BP_C" "/Game/Enemy/EnemyMeleeBT.EnemyMeleeBT" _returnvalue))
      (bind _asenemy_melee_paper_character_bp_2 (cast `/Game/Enemy/Blueprints/EnemyMeleePaperCharacter_BP` _returnvalue_3))
      (set `EnemyPaperCharacter.TypeOfEnemy` "RevivingMeleeSkeleton" _asenemy_melee_paper_character_bp_2)
      (set `EnemyPaperCharacter.behaviourActivationDelay` pBehaviourDelay _asenemy_melee_paper_character_bp_2)
      (`EnemyPaperCharacter.SetGameManager` _asenemy_melee_paper_character_bp_2 _gamemanager)
      (`EnemyPaperCharacter.Init` _asenemy_melee_paper_character_bp_2))
    (:`2`
      (bind _returnvalue_4 (`AIBlueprintHelperLibrary.SpawnAIFromClass` "/Game/Enemy/Blueprints/EnemyRangedPaperCharacter_BP.EnemyRangedPaperCharacter_BP_C" "/Game/Enemy/EnemyRangedBT.EnemyRangedBT" _returnvalue))
      (bind _asenemy_ranged_paper_character_bp (cast `/Game/Enemy/Blueprints/EnemyRangedPaperCharacter_BP` _returnvalue_4))
      (set `EnemyPaperCharacter.TypeOfEnemy` "RangedWizard" _asenemy_ranged_paper_character_bp)
      (set `EnemyPaperCharacter.behaviourActivationDelay` pBehaviourDelay _asenemy_ranged_paper_character_bp)
      (`EnemyPaperCharacter.SetGameManager` _asenemy_ranged_paper_character_bp _gamemanager)
      (`EnemyPaperCharacter.Init` _asenemy_ranged_paper_character_bp))
    (:`3`
      (bind _returnvalue_5 (`AIBlueprintHelperLibrary.SpawnAIFromClass` "/Game/Enemy/Blueprints/EnemyRangedPaperCharacter_BP.EnemyRangedPaperCharacter_BP_C" "/Game/Enemy/EnemyRangedBT.EnemyRangedBT" _returnvalue))
      (bind _asenemy_ranged_paper_character_bp_2 (cast `/Game/Enemy/Blueprints/EnemyRangedPaperCharacter_BP` _returnvalue_5))
      (set `EnemyPaperCharacter.TypeOfEnemy` "CircleAttackRangedWizard" _asenemy_ranged_paper_character_bp_2)
      (set `EnemyPaperCharacter.behaviourActivationDelay` pBehaviourDelay _asenemy_ranged_paper_character_bp_2)
      (`EnemyPaperCharacter.SetGameManager` _asenemy_ranged_paper_character_bp_2 _gamemanager)
      (`EnemyPaperCharacter.Init` _asenemy_ranged_paper_character_bp_2))))

(fn `UserConstructionScript`)