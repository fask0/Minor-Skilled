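; GameManager Blueprint that drives round and wave progression and enemy spawning from its Tick event.
; Tick polls player 0's Enter key to begin the first round, or the next wave when one is available, printing wave and round numbers.
; While a round runs with no next wave available, a Delay in Tick throttles random-spawner enemy spawns to roughly two-second intervals.
; The round, wave and spawn functions it calls are defined outside this graph.
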(event `self.ReceiveTick`
  (params (DeltaSeconds :type "Float (single-precision)"))
  (bind _returnvalue (`PlayerController.WasInputKeyJustReleased` (`GameplayStatics.GetPlayerController` 0) "Enter"))
  (if (`self.roundHasStarted`)
    (if (`self.isNextWaveAvailable`)
      (if _returnvalue
        (`self.BeginNextWave`)
        (bind _returnvalue_2 (`self.GetCurrentWave`))
        (bind _returnvalue_3 (`self.GetCurrentRound`))
        (`KismetSystemLibrary.PrintString` (`KismetStringLibrary.Concat_StrStr` "Starting W" (`KismetStringLibrary.Conv_IntToString` _returnvalue_2) "-R" (`KismetStringLibrary.Conv_IntToString` _returnvalue_3))))
      (else
        (`KismetSystemLibrary.Delay` 2.0)
        (bind _returnvalue_4 (`self.SpawnEnemyAtRandomSpawner`))
        (if _returnvalue_4
          _)))
    (elif _returnvalue
      (`self.BeginFirstRound`)
      (bind _returnvalue_5 (`self.GetCurrentWave`))
      (bind _returnvalue_6 (`self.GetCurrentRound`))
      (`KismetSystemLibrary.PrintString` (`KismetStringLibrary.Concat_StrStr` "Started W" (`KismetStringLibrary.Conv_IntToString` _returnvalue_5) "-R" (`KismetStringLibrary.Conv_IntToString` _returnvalue_6))))))

(fn `UserConstructionScript`)